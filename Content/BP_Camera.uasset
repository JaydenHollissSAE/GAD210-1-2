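; BP_Camera is a camera Blueprint that follows an enemy chosen by index.
; Every Tick it gathers all BP_Enemy actors, stores their count in EnemyAmount, and teleports the Camera to the location of the enemy at SelectedEnemy.
; The ChangeEnemy1 input compares SelectedEnemy with zero, incrementing only negative values, so it does not advance from zero or use EnemyAmount.
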(event `self.ReceiveBeginPlay`)

(event `self.ReceiveTick`
  (params (DeltaSeconds :type "Float (single-precision)"))
  (bind _outactors (`GameplayStatics.GetAllActorsOfClass` "/Game/BP_Enemy.BP_Enemy_C"))
  (set `self.EnemyAmount` (`KismetArrayLibrary.Array_Length` _outactors))
  (bind _output_get (set `self.MoveTo` (`self.K2_GetActorLocation` (`|GetArrayItem` _outactors (`self.SelectedEnemy`)))))
  (`SceneComponent.K2_SetWorldLocation` (`self.Camera`) _output_get false true))

(event `InputAction|ChangeEnemy1`
  (params (Key :type "Key Structure"))
  (bind _selectedenemy (`self.SelectedEnemy`))
  (:`Pressed`
    (`/Engine/EditorBlueprintResources/StandardMacros.CompareInt` _selectedenemy
      (:`==`
        (set `self.SelectedEnemy` 0))
      (:`<`
        (set `self.SelectedEnemy` (+ _selectedenemy 1))))))

(fn `UserConstructionScript`)